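; BP_Chain is a construction-script actor that lays instanced chain links along an editable spline, with End instances at both endpoints.
; Links are spaced by Spacing and aligned to the spline tangent.
; A second, offset set takes its roll from Rotation to form alternating links.
; The second loop is nested inside the first and also adds the endpoints, so those instances are duplicated many times.
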(event EventBeginPlay)

(event Collision|EventActorBeginOverlap
  (params (OtherActor :type Actor%20Object%20Reference)))

(event EventTick
  (params (DeltaSeconds :type Float%20%28single-precision%29)))

(fn ConstructionScript
  (Components|StaticMesh|SetStaticMesh (Variables|Default|GetChain) (Variables|Default|GetChain%20mesh))
  (for _index (range 0 (- (Math|Float|Floor (/ (Spline|GetSplineLength (Variables|Default|GetSpline)) (Variables|Default|GetSpacing))) 1))
    (Components|InstancedStaticMesh|AddInstance (Variables|Default|GetChain) (Math|Transform|MakeTransform (Spline|GetLocationatDistanceAlongSpline (Variables|Default|GetSpline) (* _index (Variables|Default|GetSpacing)) "Local") (Math|Conversions|RotationFromXVector (Spline|GetTangentatDistanceAlongSpline (Variables|Default|GetSpline) (* _index (Variables|Default|GetSpacing)) "Local")) "0.500000,0.500000,0.500000") false)
    (for _index_2 (range 0 (- (Math|Float|Floor (/ (Spline|GetSplineLength (Variables|Default|GetSpline)) (Variables|Default|GetSpacing))) 1))
      (Components|InstancedStaticMesh|AddInstance (Variables|Default|GetChain) (Math|Transform|MakeTransform (Math|Vector|MakeVector (.x (.location (Math|Transform|MakeTransform (Spline|GetLocationatDistanceAlongSpline (Variables|Default|GetSpline) (+ (* _index_2 (Variables|Default|GetSpacing)) 25.0) "Local") (Math|Rotator|MakeRotator (Variables|Default|GetRotation) (.pitch (Math|Conversions|RotationFromXVector (Spline|GetTangentatDistanceAlongSpline (Variables|Default|GetSpline) (* _index_2 (Variables|Default|GetSpacing)) "Local"))) (.yaw (Math|Conversions|RotationFromXVector (Spline|GetTangentatDistanceAlongSpline (Variables|Default|GetSpline) (* _index_2 (Variables|Default|GetSpacing)) "Local")))) "0.500000,0.500000,0.500000"))) (+ (.y (.location (Math|Transform|MakeTransform (Spline|GetLocationatDistanceAlongSpline (Variables|Default|GetSpline) (+ (* _index_2 (Variables|Default|GetSpacing)) 25.0) "Local") (Math|Rotator|MakeRotator (Variables|Default|GetRotation) (.pitch (Math|Conversions|RotationFromXVector (Spline|GetTangentatDistanceAlongSpline (Variables|Default|GetSpline) (* _index_2 (Variables|Default|GetSpacing)) "Local"))) (.yaw (Math|Conversions|RotationFromXVector (Spline|GetTangentatDistanceAlongSpline (Variables|Default|GetSpline) (* _index_2 (Variables|Default|GetSpacing)) "Local")))) "0.500000,0.500000,0.500000"))) -7.0) (+ (.z (.location (Math|Transform|MakeTransform (Spline|GetLocationatDistanceAlongSpline (Variables|Default|GetSpline) (+ (* _index_2 (Variables|Default|GetSpacing)) 25.0) "Local") (Math|Rotator|MakeRotator (Variables|Default|GetRotation) (.pitch (Math|Conversions|RotationFromXVector (Spline|GetTangentatDistanceAlongSpline (Variables|Default|GetSpline) (* _index_2 (Variables|Default|GetSpacing)) "Local"))) (.yaw (Math|Conversions|RotationFromXVector (Spline|GetTangentatDistanceAlongSpline (Variables|Default|GetSpline) (* _index_2 (Variables|Default|GetSpacing)) "Local")))) "0.500000,0.500000,0.500000"))) 1e+01)) (.rotation (Math|Transform|MakeTransform (Spline|GetLocationatDistanceAlongSpline (Variables|Default|GetSpline) (+ (* _index_2 (Variables|Default|GetSpacing)) 25.0) "Local") (Math|Rotator|MakeRotator (Variables|Default|GetRotation) (.pitch (Math|Conversions|RotationFromXVector (Spline|GetTangentatDistanceAlongSpline (Variables|Default|GetSpline) (* _index_2 (Variables|Default|GetSpacing)) "Local"))) (.yaw (Math|Conversions|RotationFromXVector (Spline|GetTangentatDistanceAlongSpline (Variables|Default|GetSpline) (* _index_2 (Variables|Default|GetSpacing)) "Local")))) "0.500000,0.500000,0.500000")) (.scale (Math|Transform|MakeTransform (Spline|GetLocationatDistanceAlongSpline (Variables|Default|GetSpline) (+ (* _index_2 (Variables|Default|GetSpacing)) 25.0) "Local") (Math|Rotator|MakeRotator (Variables|Default|GetRotation) (.pitch (Math|Conversions|RotationFromXVector (Spline|GetTangentatDistanceAlongSpline (Variables|Default|GetSpline) (* _index_2 (Variables|Default|GetSpacing)) "Local"))) (.yaw (Math|Conversions|RotationFromXVector (Spline|GetTangentatDistanceAlongSpline (Variables|Default|GetSpline) (* _index_2 (Variables|Default|GetSpacing)) "Local")))) "0.500000,0.500000,0.500000"))) false)
      (Components|InstancedStaticMesh|AddInstance (Variables|Default|GetEnd) (Math|Transform|MakeTransform (Spline|GetLocationatSplinePoint (Variables|Default|GetSpline) (- (Spline|GetNumberOfSplinePoints (Variables|Default|GetSpline)) 1) "Local") "0, 0, 0" "0.750000,0.750000,0.750000") false)
      (Components|InstancedStaticMesh|AddInstance (Variables|Default|GetEnd) (Math|Transform|MakeTransform (Spline|GetLocationatSplinePoint (Variables|Default|GetSpline) 0 "Local") "0, 0, 0" "0.750000,0.750000,0.750000") false))))