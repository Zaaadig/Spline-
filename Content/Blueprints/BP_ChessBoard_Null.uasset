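; BP_ChessBoard_Null is an actor Blueprint that builds a grid of stone mesh instances in its construction script.
; It clears its InstancedStaticMesh, assigns SMStone, then nested loops add instances 100 units apart, with VarY along local X and VarX along Z, forming an upright grid.
; Each cell prints a debug string and passes an always-true branch, so no checker alternation occurs.
; The event graph holds only disabled stubs.
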(event EventBeginPlay)

(event Collision|EventActorBeginOverlap
  (params (OtherActor :type Actor%20Object%20Reference)))

(event EventTick
  (params (DeltaSeconds :type Float%20%28single-precision%29)))

(fn ConstructionScript
  (Components|InstancedStaticMesh|ClearInstances (Variables|Default|GetInstancedStaticMesh))
  (Components|StaticMesh|SetStaticMesh (Variables|Default|GetInstancedStaticMesh) (Variables|Default|GetSM_Stone))
  (for _index (range 0 (- (Variables|Default|GetVarX) 1))
    (for _index_2 (range 0 (- (Variables|Default|GetVarY) 1))
      (Development|PrintString "Hello")
      (if true
        (Components|InstancedStaticMesh|AddInstance (Variables|Default|GetInstancedStaticMesh) (Math|Transform|MakeTransform (Math|Vector|MakeVector (Math|Conversions|ToFloat(Integer) (* _index_2 100)) 0.0 (Math|Conversions|ToFloat(Integer) (* _index 100)))) false)))))