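; BP_ChessBoard builds a vertical chessboard-style grid of stone mesh instances in the local XZ plane, sized by VarX rows and VarY columns.
; The construction script rebuilds one InstancedStaticMesh and records instance indices in AllInstance.
; Per-instance custom data feeds the material a 0/1 value from row plus instance index parity, checkered only for even VarY.
; Each custom-data write result is printed for debugging.
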(event EventBeginPlay)

(fn ConstructionScript
  (bind _instancedstaticmesh (Variables|Default|GetInstancedStaticMesh))
  (Components|InstancedStaticMesh|ClearInstances (Variables|Default|GetInstancedStaticMesh))
  (Utilities|Array|Clear (Variables|Default|GetAllInstance))
  (Components|StaticMesh|SetStaticMesh _instancedstaticmesh (Variables|Default|GetSM_Stone))
  (Rendering|Material|SetMaterial _instancedstaticmesh 0 "/Game/Blueprints/BP_ChessBoard/M_PerInstanceCustomData.M_PerInstanceCustomData")
  (for _index (range 0 (- (Variables|Default|GetVarX) 1))
    (for _index_2 (range 0 (- (Variables|Default|GetVarY) 1))
      (bind _returnvalue (Components|InstancedStaticMesh|AddInstance (Variables|Default|GetInstancedStaticMesh) (Math|Transform|MakeTransform (Math|Vector|MakeVector (Math|Conversions|ToFloat(Integer) (* _index_2 100)) 0.0 (Math|Conversions|ToFloat(Integer) (* _index 100)))) false))
      (Utilities|Array|Add (Variables|Default|GetAllInstance) _returnvalue)
      (bind _returnvalue_2 (Components|InstancedStaticMesh|SetCustomDataValue (Variables|Default|GetInstancedStaticMesh) _returnvalue 0 (Math|Conversions|ToFloat(Boolean) (== (Math|Integer|%(Integer) (+ _index _returnvalue) 2) 0)) false))
      (Development|PrintString (Utilities|String|ToString(Boolean) _returnvalue_2)))))