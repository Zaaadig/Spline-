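; BP_Laser is a laser actor whose capsule spans a Start and an End component, with no active event logic.
; The construction script moves End to LaserEndLocation, then rotates the capsule along the line between the two points using a look-at rotation combined with a 90-degree offset.
; It places the capsule at half the Start-to-End vector, using that vector's length as half-height and CapsuleRadius as thickness.
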(event EventBeginPlay)

(event Collision|EventActorBeginOverlap
  (params (OtherActor :type Actor%20Object%20Reference)))

(event EventTick
  (params (DeltaSeconds :type Float%20%28single-precision%29)))

(fn ConstructionScript
  (bind _start (Variables|Default|GetStart))
  (bind _end (Variables|Default|GetEnd))
  (bind _relativelocation (Variables|/Script/Engine.SceneComponent|GetRelativeLocation _end))
  (bind _relativelocation_2 (Variables|/Script/Engine.SceneComponent|GetRelativeLocation _start))
  (Utilities|FlowControl|Sequence
    (:then_0
      (Transformation|SetRelativeLocation (Variables|Default|GetEnd) (Variables|Default|GetLaser%20End%20Location) false false)
      (bind _output_get (Variables|Default|SetMid%20Location (/ (- _relativelocation _relativelocation_2) 2.0)))
      (Transformation|SetRelativeLocationAndRotation (Variables|Default|GetCapsule) _output_get (Math|Rotator|CombineRotators "90.000000,0.000000,0.000000" (Math|Rotator|FindLookatRotation _relativelocation_2 _relativelocation)) false false)
      (Components|Capsule|SetCapsuleHalfHeight (Variables|Default|GetCapsule) (Math|Vector|VectorLength (Variables|Default|GetMid%20Location)) true)
      (Components|Capsule|SetCapsuleRadius (Variables|Default|GetCapsule) (Variables|Default|GetCapsule%20Radius) true))))