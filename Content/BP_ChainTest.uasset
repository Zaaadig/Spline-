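; BP_ChainTest is a test actor that builds a chain along a spline in its construction script.
; It places scaled ChainMesh instances on the Start component at Spacing intervals, following spline pitch and yaw and alternating 90-degree roll to interlock links.
; The End component gets instances at both spline endpoints, re-added on every loop iteration, so they stack.
; The event graph has no logic.
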(event EventBeginPlay)

(event Collision|EventActorBeginOverlap
  (params (OtherActor :type Actor%20Object%20Reference)))

(event EventTick
  (params (DeltaSeconds :type Float%20%28single-precision%29)))

(fn ConstructionScript
  (Components|StaticMesh|SetStaticMesh (Variables|Default|GetStart) (Variables|Default|GetChain%20mesh))
  (for _index (range 0 (- (Math|Float|Floor (/ (Spline|GetSplineLength (Variables|Default|GetSpline)) (Variables|Default|GetSpacing))) 1))
    (Components|InstancedStaticMesh|AddInstance (Variables|Default|GetStart) (Math|Transform|MakeTransform (.location (Spline|GetTransformatDistanceAlongSpline (Variables|Default|GetSpline) (* _index (Variables|Default|GetSpacing)) "Local" false)) (Math|Rotator|MakeRotator (select (== (Math|Integer|%(Integer) _index 2) 0) 9e+01 0.0) (.pitch (.rotation (Spline|GetTransformatDistanceAlongSpline (Variables|Default|GetSpline) (* _index (Variables|Default|GetSpacing)) "Local" false))) (.yaw (.rotation (Spline|GetTransformatDistanceAlongSpline (Variables|Default|GetSpline) (* _index (Variables|Default|GetSpacing)) "Local" false)))) "0.750000,0.750000,0.750000") false)
    (Components|InstancedStaticMesh|AddInstance (Variables|Default|GetEnd) (Math|Transform|MakeTransform (Spline|GetLocationatSplinePoint (Variables|Default|GetSpline) (- (Spline|GetNumberOfSplinePoints (Variables|Default|GetSpline)) 1) "Local")) false)
    (Components|InstancedStaticMesh|AddInstance (Variables|Default|GetEnd) (Math|Transform|MakeTransform (Spline|GetLocationatSplinePoint (Variables|Default|GetSpline) 0 "Local")) false)))