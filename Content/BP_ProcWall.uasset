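; BP_ProcWall is a procedural wall actor built from a grid of instanced static meshes with randomized depth.
; The construction script assigns the mesh and, when Activer is set, lays out VarX by VarY instances in the local YZ plane using cube length and offset.
; BeginPlay randomizes each instance's X scale.
; With Alligner set, it also shifts instances along X to compensate for scale, re-running that pass inside the randomizing loop.
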(event EventBeginPlay
  (for _index (range 0 (- (Components|InstancedStaticMesh|GetInstanceCount (Variables|Default|GetInstancedStaticMesh)) 1))
    (Components|InstancedStaticMesh|UpdateInstanceTransform (Variables|Default|GetInstancedStaticMesh) _index (Math|Transform|MakeTransform (.location (.OutInstanceTransform (Components|InstancedStaticMesh|GetInstanceTransform (Variables|Default|GetInstancedStaticMesh) _index false))) (.rotation (.OutInstanceTransform (Components|InstancedStaticMesh|GetInstanceTransform (Variables|Default|GetInstancedStaticMesh) _index false))) (Math|Vector|MakeVector (Math|Random|RandomFloatinRange (Variables|Default|GetScale%20Min) (Variables|Default|GetMax)) 1.0 1.0)) false false false)
    (if (Variables|Default|GetAlligner%20?)
      (for _index_2 (range 0 (- (Components|InstancedStaticMesh|GetInstanceCount (Variables|Default|GetInstancedStaticMesh)) 1))
        (Components|InstancedStaticMesh|UpdateInstanceTransform (Variables|Default|GetInstancedStaticMesh) _index_2 (Math|Transform|MakeTransform (Math|Vector|MakeVector (* (- 1.0 (.x (.Scale (Math|Transform|BreakTransform (.OutInstanceTransform (Components|InstancedStaticMesh|GetInstanceTransform (Variables|Default|GetInstancedStaticMesh) _index_2 false)))))) 5e+01) (.y (.Location (Math|Transform|BreakTransform (.OutInstanceTransform (Components|InstancedStaticMesh|GetInstanceTransform (Variables|Default|GetInstancedStaticMesh) _index_2 false))))) (.z (.Location (Math|Transform|BreakTransform (.OutInstanceTransform (Components|InstancedStaticMesh|GetInstanceTransform (Variables|Default|GetInstancedStaticMesh) _index_2 false)))))) (.Rotation (Math|Transform|BreakTransform (.OutInstanceTransform (Components|InstancedStaticMesh|GetInstanceTransform (Variables|Default|GetInstancedStaticMesh) _index_2 false)))) (Math|Vector|MakeVector (.x (.Scale (Math|Transform|BreakTransform (.OutInstanceTransform (Components|InstancedStaticMesh|GetInstanceTransform (Variables|Default|GetInstancedStaticMesh) _index_2 false))))) 1.0 1.0)) false false false)))))

(event Collision|EventActorBeginOverlap
  (params (OtherActor :type Actor%20Object%20Reference)))

(fn ConstructionScript
  (Components|StaticMesh|SetStaticMesh (Variables|Default|GetInstancedStaticMesh) (Variables|Default|GetISM))
  (if (Variables|Default|GetActiver)
    (for _index (range 0 (+ (Variables|Default|GetVar%20Y) -1))
      (for _index_2 (range 0 (+ (Variables|Default|GetVar%20X) -1))
        (Components|InstancedStaticMesh|AddInstance (Variables|Default|GetInstancedStaticMesh) (Math|Transform|MakeTransform (Math|Vector|MakeVector 0.0 (Math|Conversions|ToFloat(Integer) (+ (* _index_2 (Variables|Default|GetLenghtOfCube)) (Variables|Default|GetDecal))) (Math|Conversions|ToFloat(Integer) (+ (* _index (Variables|Default|GetLenghtOfCube)) (Variables|Default|GetDecal)))) "0, 0, 0" (Math|Vector|MakeVector 1.0 1.0 1.0)) false)))))